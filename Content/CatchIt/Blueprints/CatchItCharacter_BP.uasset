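; Player character for the CatchIt game, moving sideways and showing the HUD and game-over screen.
; BeginPlay adds the Enhanced Input mapping context and creates the HUD widget; the move action drives movement along the control rotation's right vector.
; Tick polls Lives and, at zero or below, adds a game-over widget every frame with no guard, showing the cursor and switching to UI-only input.
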(event `self.ReceiveBeginPlay`
  ;[0 0.8602 1] Event Begin Play
  (bind _asplayer_controller (cast `PlayerController` (`self.GetController`)))
  (bind _returnvalue (pcsubsystem `EnhancedInputLocalPlayerSubsystem` _asplayer_controller))
  (`/Engine/EditorBlueprintResources/StandardMacros.IsValid` _returnvalue
    (:`Is Valid`
      (`EnhancedInputSubsystemInterface.AddMappingContext` _returnvalue "/Game/CatchIt/Inputs/CatchIt_IMC.CatchIt_IMC" 0 (struct))
      (bind _returnvalue_2 (`|CreateWidget` "/Game/CatchIt/Blueprints/CatchItHUD_WB.CatchItHUD_WB_C"))
      (bind _output_get (set `self.PlayerHUD` _returnvalue_2))
      (`UserWidget.AddToViewport` _output_get 0))))

(event `EnhancedInput|/Game/CatchIt/Inputs/CatchItMove_IA`
  (params (ActionValue :type "Vector2D Structure") (ElapsedSeconds :type "Float (double-precision)") (TriggeredSeconds :type "Float (double-precision)") (InputAction :type "InputAction Object Reference" :default "/Game/CatchIt/Inputs/CatchItMove_IA.CatchItMove_IA"))
  (bind (_returnvalue_roll _returnvalue_pitch _returnvalue_yaw) (`KismetMathLibrary.BreakRotator` (`self.GetControlRotation`)))
  ;[1 0.9146 0] Move Input
  (:`Triggered`
    (`self.AddMovementInput` (`KismetMathLibrary.GetRightVector` (`KismetMathLibrary.MakeRotator` _returnvalue_roll 0.0 _returnvalue_yaw)) ActionValue_X)))

(event `self.ReceiveTick`
  (params (DeltaSeconds :type "Float (single-precision)"))
  (bind _returnvalue (`GameplayStatics.GetPlayerController` 0))
  (if (<= (`self.Lives`) 0)
    (bind _returnvalue_2 (`|CreateWidget` "/Game/CatchIt/Blueprints/CatchItGameOver_BP.CatchItGameOver_BP_C"))
    (`UserWidget.AddToViewport` _returnvalue_2 0)
    (set `PlayerController.bShowMouseCursor` true _returnvalue)
    (`WidgetBlueprintLibrary.SetInputMode_UIOnlyEx` _returnvalue null)))

(fn `UserConstructionScript`)