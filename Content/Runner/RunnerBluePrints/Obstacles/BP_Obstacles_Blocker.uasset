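; BP_Obstacles_Blocker is a runner obstacle that kills the player unless they are sliding under or through it.
; On actor overlap it casts the other actor to BP_RunnerCharacter and checks IsSliding.
; If the character is not sliding, it calls Death on the character, waits a short delay, then pauses the game.
; The overlap does not call the parent implementation, and the construction script only runs the parent's.
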(event `self.ReceiveActorBeginOverlap`
  (params (OtherActor :type "Actor Object Reference"))
  (bind _asbp_runner_character (cast `/Game/Runner/RunnerBluePrints/CharactersBps/BP_RunnerCharacter` OtherActor))
  (if (not (`/Game/Runner/RunnerBluePrints/CharactersBps/BP_RunnerCharacter.isSliding?` _asbp_runner_character))
    (`/Game/Runner/RunnerBluePrints/CharactersBps/BP_RunnerCharacter.Death` _asbp_runner_character)
    (`KismetSystemLibrary.Delay` 1.0)
    (`GameplayStatics.SetGamePaused` true)))

(fn `UserConstructionScript`
  (`parent.UserConstructionScript`))