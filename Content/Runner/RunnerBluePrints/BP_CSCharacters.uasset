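; Character selection Blueprint for the runner game, previewing Manny, Kevin and Gideon and committing the chosen one.
; Show events toggle hidden-in-game so only one character is visible at a time.
; Despite their names, Spawn events spawn nothing: they pass the matching runner pawn to SaveCharacter.
; SaveCharacter loads or creates the Runner_SaveGame in the PlayerCharacter slot, stores the choice, then opens Runner_Map.
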(event `ShowManny`
  (`SceneComponent.SetHiddenInGame` (`self.Manny`) false false)
  (`SceneComponent.SetHiddenInGame` (`self.Kevin`) true false)
  (`SceneComponent.SetHiddenInGame` (`self.Gideon`) true false))

(event `ShowKevin`
  (`SceneComponent.SetHiddenInGame` (`self.Manny`) true false)
  (`SceneComponent.SetHiddenInGame` (`self.Kevin`) false false)
  (`SceneComponent.SetHiddenInGame` (`self.Gideon`) true false))

(event `ShowGideon`
  (`SceneComponent.SetHiddenInGame` (`self.Manny`) true false)
  (`SceneComponent.SetHiddenInGame` (`self.Kevin`) true false)
  (`SceneComponent.SetHiddenInGame` (`self.Gideon`) false false))

(event `SpawnManny`
  (bind _aspawn (castclass `Pawn` "/Game/Runner/RunnerBluePrints/CharactersBps/BP_RunnerCharacter.BP_RunnerCharacter_C"))
  (bind _output_get (set `self.As Pawn` _aspawn))
  (`self.SaveCharacter` _output_get))

(event `SpawnKevin`
  (bind _aspawn (castclass `Pawn` "/Game/Runner/RunnerBluePrints/CharactersBps/BP_RunnerKevin.BP_RunnerKevin_C"))
  (bind _output_get (set `self.As Pawn` _aspawn))
  (`self.SaveCharacter` _output_get))

(event `SpawnGideon`
  (bind _aspawn (castclass `Pawn` "/Game/Runner/RunnerBluePrints/CharactersBps/BP_RunnerGideon.BP_RunnerGideon_C"))
  (bind _output_get (set `self.As Pawn` _aspawn))
  (`self.SaveCharacter` _output_get))

(fn `SaveCharacter`
  (params (PlayerCharacter :type "Pawn Class Reference"))
  (bind _returnvalue (`GameplayStatics.DoesSaveGameExist` "PlayerCharacter"))
  (if _returnvalue
    (bind _returnvalue_2 (`GameplayStatics.LoadGameFromSlot` "PlayerCharacter"))
    (bind _output_get (set `self.SaverSubClass` _returnvalue_2))
    (bind _asrunner_save_game (cast `/Game/Runner/RunnerBluePrints/Runner_SaveGame` _output_get))
    (set `/Game/Runner/RunnerBluePrints/Runner_SaveGame.PlayerCharacter` PlayerCharacter _asrunner_save_game)
    (`GameplayStatics.SaveGameToSlot` (`self.SaverSubClass`) "PlayerCharacter")
    (else
      (bind _returnvalue_3 (`GameplayStatics.CreateSaveGameObject` "/Game/Runner/RunnerBluePrints/Runner_SaveGame.Runner_SaveGame_C"))
      (bind _output_get_2 (set `self.SaverSubClass` _returnvalue_3))
      (bind _asrunner_save_game_2 (cast `/Game/Runner/RunnerBluePrints/Runner_SaveGame` _output_get_2))
      (set `/Game/Runner/RunnerBluePrints/Runner_SaveGame.PlayerCharacter` PlayerCharacter _asrunner_save_game_2)
      (`GameplayStatics.SaveGameToSlot` (`self.SaverSubClass`) "PlayerCharacter")))
  (`GameplayStatics.OpenLevelBySoftObjectPtr` "/Game/Runner/RunnerMaps/Runner_Map.Runner_Map"))

(fn `UserConstructionScript`)