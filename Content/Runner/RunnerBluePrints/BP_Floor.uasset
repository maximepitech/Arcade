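; Floor tile for an endless runner that fills its lanes with random obstacles, coins and periodic power-ups.
; The construction script builds arrow spawn points per lane, shuffles them and attaches child actors, adding a power-up when the game mode's FloorCount exceeds a threshold, then resetting it.
; Box overlap asks BP_RunnerGameMode to extend the floor, nudges player speed up within a clamp and adds multiplier-based points.
; GetAttachPoint exposes the arrow transform.
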(event `self.Box.OnComponentBeginOverlap`
  (params (OverlappedComponent :type "PrimitiveComponent Object Reference") (OtherActor :type "Actor Object Reference") (OtherComp :type "PrimitiveComponent Object Reference") (OtherBodyIndex :type Integer) (bFromSweep :type Boolean) (SweepResult :type "HitResult Structure (by ref)"))
  ;[1 1 1] Extend Floor
  (bind _asbp_runner_game_mode (cast `/Game/Runner/RunnerBluePrints/BP_RunnerGameMode` (`GameplayStatics.GetGameMode`)))
  (`/Game/Runner/RunnerBluePrints/BP_RunnerGameMode.ExtendFloor` _asbp_runner_game_mode)
  ;[1 1 1] Change Speed
  (bind _asbp_runner_character (cast `/Game/Runner/RunnerBluePrints/CharactersBps/BP_RunnerCharacter` (`GameplayStatics.GetPlayerCharacter` 0)))
  (bind _charactermovement (`Character.CharacterMovement` _asbp_runner_character))
  (set `CharacterMovementComponent.MaxWalkSpeed` (`KismetMathLibrary.FClamp` (* (`CharacterMovementComponent.MaxWalkSpeed` _charactermovement) 1.001) 700.0 1500.0) _charactermovement)
  ;[1 1 1] Set Current Score
  (bind _asbp_runner_game_mode_2 (cast `/Game/Runner/RunnerBluePrints/BP_RunnerGameMode` (`GameplayStatics.GetGameMode`)))
  (set `/Game/Runner/RunnerBluePrints/BP_RunnerGameMode.CurrentPoints` (+ (* (`/Game/Runner/RunnerBluePrints/BP_RunnerGameMode.PointsMulti` _asbp_runner_game_mode_2) 1) (`/Game/Runner/RunnerBluePrints/BP_RunnerGameMode.CurrentPoints` _asbp_runner_game_mode_2)) _asbp_runner_game_mode_2))

(fn `CoinSpawnPoints`
  (for _array_element (`self.LanePosition`)
    (for _index (range 10)
      (bind _returnvalue (`AddComponent|NODE_AddArrowComponent-1` :`RelativeTransform` (`KismetMathLibrary.MakeTransform` (`KismetMathLibrary.MakeVector` (* _index 75.0) _array_element))))
      (`ArrowComponent.SetArrowColor` _returnvalue (struct :`R` 0.050797 :`B` 1.0 :`A` 1.0))
      (`KismetArrayLibrary.Array_Add` (`self.CSpawnPoints`) (`SceneComponent.K2_GetComponentToWorld` _returnvalue)))))

(fn `GetAttachPoint`
  (returns (ReturnValue :type "Transform Structure"))
  (return (`SceneComponent.K2_GetComponentToWorld` (`self.Arrow`))))

(fn `PowerUpsSpawnPoints`
  (for _array_element (`self.LanePosition`)
    (for _index (range 1 3)
      (bind _returnvalue (`AddComponent|NODE_AddArrowComponent-2` :`RelativeTransform` (`KismetMathLibrary.MakeTransform` (`KismetMathLibrary.MakeVector` (* _index 250.0) _array_element))))
      (`ArrowComponent.SetArrowColor` _returnvalue (struct :`R` 0.136643 :`G` 1.0 :`A` 1.0))
      (`KismetArrayLibrary.Array_Add` (`self.PSpawnPoints`) (`SceneComponent.K2_GetComponentToWorld` _returnvalue)))))

(fn `SetupSpawnPoint`
  (for _array_element (`self.LanePosition`)
    (for _index (range 2)
      (bind _returnvalue (`AddComponent|NODE_AddArrowComponent-0` :`RelativeTransform` (`KismetMathLibrary.MakeTransform` (`KismetMathLibrary.MakeVector` (* _index 650.0) _array_element))))
      (`KismetArrayLibrary.Array_Add` (`self.SpawnPoints`) (`SceneComponent.K2_GetComponentToWorld` _returnvalue)))))

(fn `SpawnCoins`
  (locals (RandomSpawnPoints :type "Array of Transform Structure"))
  (bind _output_get (set `local.RandomSpawnPoints` (`self.CSpawnPoints`)))
  (`KismetArrayLibrary.Array_Shuffle` _output_get)
  (for _index (range (+ (`KismetMathLibrary.RandomIntegerInRange` 5 9) 1))
    (switch `int` 0
      (:`0`
        (`AddComponent|NODE_AddChildActorComponent-7` :`RelativeTransform` (`KismetMathLibrary.MakeRelativeTransform` (`|GetArrayItem` (`local.RandomSpawnPoints`) _index) (`self.GetTransform`)))))))

(fn `SpawnObstacles`
  (locals (RandomSpawnPoints :type "Array of Transform Structure"))
  (bind _output_get (set `local.RandomSpawnPoints` (`self.SpawnPoints`)))
  (`KismetArrayLibrary.Array_Shuffle` _output_get)
  (for _index (range (+ (`KismetMathLibrary.RandomIntegerInRange` 0 1) 1))
    (switch `int` (`KismetMathLibrary.RandomIntegerInRange` 0 1)
      (:`0`
        (bind _returnvalue (`KismetMathLibrary.MakeRelativeTransform` (`|GetArrayItem` (`local.RandomSpawnPoints`) _index) (`self.GetTransform`)))
        (`AddComponent|NODE_AddChildActorComponent-0` :`RelativeTransform` _returnvalue))
      (:`1`
        (`AddComponent|NODE_AddChildActorComponent-1` :`RelativeTransform` _returnvalue)))))

(fn `SpawnPowerUps`
  (locals (RandomSpawnPoints :type "Array of Transform Structure"))
  (bind _asbp_runner_game_mode (cast `/Game/Runner/RunnerBluePrints/BP_RunnerGameMode` (`GameplayStatics.GetGameMode`)))
  (if (> (`/Game/Runner/RunnerBluePrints/BP_RunnerGameMode.FloorCount` _asbp_runner_game_mode) 10)
    (bind _output_get (set `local.RandomSpawnPoints` (`self.PSpawnPoints`)))
    (`KismetArrayLibrary.Array_Shuffle` _output_get)
    (`AddComponent|NODE_AddChildActorComponent-8` :`RelativeTransform` (`KismetMathLibrary.MakeRelativeTransform` (`|GetArrayItem` (`local.RandomSpawnPoints`)) (`self.GetTransform`)))
    (set `/Game/Runner/RunnerBluePrints/BP_RunnerGameMode.FloorCount` 0 _asbp_runner_game_mode)))

(fn `UserConstructionScript`
  (`self.SetupSpawnPoint`)
  (`self.SpawnObstacles`)
  (`self.CoinSpawnPoints`)
  (`self.SpawnCoins`)
  (`self.PowerUpsSpawnPoints`)
  (`self.SpawnPowerUps`))