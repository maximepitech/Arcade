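; Game mode for a runner game that builds a continuous track of BP_Floor tiles and holds the coin count.
; On BeginPlay it spawns the starting tiles, reloading Coins from the CoinValue save slot on each loop iteration.
; Each tile supplies the attach point where the next one spawns.
; ExtendFloor appends a tile and destroys the oldest once the array exceeds NumberOfTiles plus a fixed buffer.
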(event `self.ReceiveBeginPlay`
  (for _ (range (`self.NumberOfTiles`))
    (`self.AddFloor`)
    (bind _returnvalue (`GameplayStatics.LoadGameFromSlot` "CoinValue"))
    (bind _asrunner_save_game (cast `/Game/Runner/RunnerBluePrints/Runner_SaveGame` _returnvalue))
    (set `self.Coins` (`/Game/Runner/RunnerBluePrints/Runner_SaveGame.CoinValue` _asrunner_save_game))))

(fn `AddFloor`
  (bind _returnvalue (`|SpawnActorFromClass` "/Game/Runner/RunnerBluePrints/BP_Floor.BP_Floor_C" (`self.FloorAttachPoint`) "Undefined" "MultiplyWithRoot" null null))
  (bind _returnvalue_2 (`/Game/Runner/RunnerBluePrints/BP_Floor.GetAttachPoint` _returnvalue))
  (set `self.FloorAttachPoint` _returnvalue_2)
  (`KismetArrayLibrary.Array_Add` (`self.FloorTiles`) _returnvalue)
  (bind _result (`/Engine/EditorBlueprintResources/StandardMacros.IncrementInt` (`self.FloorCount`))
    (:`  `
      (set `self.FloorCount` _result))))

(fn `ExtendFloor`
  (bind _floortiles (`self.FloorTiles`))
  (bind _output (`|GetArrayItem` _floortiles))
  (`self.AddFloor`)
  (if (> (`KismetArrayLibrary.Array_Length` (`self.FloorTiles`)) (+ (`self.NumberOfTiles`) 10))
    (`self.K2_DestroyActor` _output)
    (`KismetArrayLibrary.Array_RemoveItem` _floortiles _output)))

(fn `UserConstructionScript`)