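; Brick actor for a Brick Breaker game that loses strength on each ball hit and shows its remaining strength by glow color.
; The construction script and non-lethal hits call UpdateBrickColor to swap the cube material between red, yellow and green.
; At zero strength it plays a sound and explosion, destroys itself, then checks for remaining bricks.
; When none remain, LevelTracker_BP's level index decides between opening level 2 or showing the win widget.
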(event `self.ReceiveHit`
  (params (MyComp :type "PrimitiveComponent Object Reference") (Other :type "Actor Object Reference") (OtherComp :type "PrimitiveComponent Object Reference") (bSelfMoved :type Boolean) (HitLocation :type "Vector Structure") (HitNormal :type "Vector Structure") (NormalImpulse :type "Vector Structure") (Hit :type "HitResult Structure (by ref)"))
  (cast `/Game/BrickBreaker/Blueprints/BrickBreakerBall_BP` Other)
  (bind _result (`/Engine/EditorBlueprintResources/StandardMacros.DecrementInt` (`self.BrickStrength`))
    (:`  `
      (if (== _result 0)
        (`GameplayStatics.PlaySoundAtLocation` "/Game/BrickBreaker/SFX/break.break" (`self.K2_GetActorLocation`) (struct) 1.0 1.0 0.0 null null null null)
        (`GameplayStatics.SpawnEmitterAtLocation` "/Game/StarterContent/Particles/P_Explosion.P_Explosion" (`self.K2_GetActorLocation`))
        (`self.K2_DestroyActor`)
        (bind _outactors (`GameplayStatics.GetAllActorsOfClass` "Brick_BP_C"))
        (if (== (`KismetArrayLibrary.Array_Length` _outactors) 0)
          (bind _returnvalue (`GameplayStatics.GetActorOfClass` "/Game/BrickBreaker/Blueprints/LevelTracker_BP.LevelTracker_BP_C"))
          (switch `int` (`/Game/BrickBreaker/Blueprints/LevelTracker_BP.LevelIndex` _returnvalue)
            (:`1`
              (`GameplayStatics.OpenLevelBySoftObjectPtr` "/Game/BrickBreaker/Maps/BrickBreakerLevel2_Map.BrickBreakerLevel2_Map"))
            (:`2`
              (bind _returnvalue_2 (`|CreateWidget` "/Game/BrickBreaker/Blueprints/BrickBreakerWin_WB.BrickBreakerWin_WB_C"))
              (`UserWidget.AddToViewport` _returnvalue_2 0))))
        (else
          (`self.UpdateBrickColor`))))))

(fn `UpdateBrickColor`
  (bind _cube (`self.Cube`))
  (switch `int` (`self.BrickStrength`)
    (:`1`
      (`PrimitiveComponent.SetMaterial` _cube 0 "/Game/BrickBreaker/Materials/GlowRed_MAT_Inst.GlowRed_MAT_Inst"))
    (:`2`
      (`PrimitiveComponent.SetMaterial` _cube 0 "/Game/BrickBreaker/Materials/GlowYellow_MAT_Inst.GlowYellow_MAT_Inst"))
    (:`3`
      (`PrimitiveComponent.SetMaterial` _cube 0 "/Game/BrickBreaker/Materials/GlowGreen_MAT_Inst.GlowGreen_MAT_Inst"))))

(fn `UserConstructionScript`
  (`self.UpdateBrickColor`))