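; Player-controlled paddle for the BrickBreaker game.
; On BeginPlay it registers the Enhanced Input mapping context, creates and shows the player HUD, hides the cursor and switches to game-only input.
; The move action offsets the paddle component along its local Z by input times PaddleSpeed, swept for collision and not scaled by delta time.
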(event `self.ReceiveBeginPlay`
  (bind _returnvalue (`GameplayStatics.GetPlayerController` 0))
  ;[1 1 1] EventBeginPlay / Add Inputs
  (bind _asplayer_controller (cast `PlayerController` (`self.GetController`)))
  (bind _returnvalue_2 (pcsubsystem `EnhancedInputLocalPlayerSubsystem` _asplayer_controller))
  (`/Engine/EditorBlueprintResources/StandardMacros.IsValid` _returnvalue_2
    (:`Is Valid`
      (`EnhancedInputSubsystemInterface.AddMappingContext` _returnvalue_2 "/Game/BrickBreaker/Inputs/BrickBreaker_IMC.BrickBreaker_IMC" 0 (struct))
      (bind _returnvalue_3 (`|CreateWidget` "/Game/BrickBreaker/Blueprints/BrickBeakerPlayerHud_WP.BrickBeakerPlayerHud_WP_C"))
      (bind _output_get (set `self.PlayerHud` _returnvalue_3))
      (`UserWidget.AddToViewport` _output_get 0)
      (set `PlayerController.bShowMouseCursor` false _returnvalue)
      (`WidgetBlueprintLibrary.SetInputMode_GameOnly` _returnvalue))))

(event `EnhancedInput|/Game/BrickBreaker/Inputs/BrickBreakerMove_IA`
  (params (ActionValue :type "Float (double-precision)") (ElapsedSeconds :type "Float (double-precision)") (TriggeredSeconds :type "Float (double-precision)") (InputAction :type "InputAction Object Reference" :default "/Game/BrickBreaker/Inputs/BrickBreakerMove_IA.BrickBreakerMove_IA"))
  ;[1 1 1] Input Move
  (:`Triggered`
    (`SceneComponent.K2_AddLocalOffset` (`self.Paddle`) (`KismetMathLibrary.MakeVector` 0.0 0.0 (* ActionValue (`self.PaddleSpeed`))) true false)))

(fn `UserConstructionScript`)