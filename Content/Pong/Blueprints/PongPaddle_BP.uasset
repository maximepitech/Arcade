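; PongPaddle_BP is the player-controlled paddle in the Pong game.
; On BeginPlay it sets game-only input, adds the Pong Enhanced Input mapping context to the local player, then creates and displays the score widget, keeping it as ScoreHUD.
; The move input action slides the Cube component along its local Y axis, scaled by PlayerSpeed, with a sweep so collisions block it.
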(event `self.ReceiveBeginPlay`
  (`WidgetBlueprintLibrary.SetInputMode_GameOnly` (`GameplayStatics.GetPlayerController` 0))
  (bind _asplayer_controller (cast `PlayerController` (`self.GetController`)))
  (bind _returnvalue (pcsubsystem `EnhancedInputLocalPlayerSubsystem` _asplayer_controller))
  (`/Engine/EditorBlueprintResources/StandardMacros.IsValid` _returnvalue
    (:`Is Valid`
      (`EnhancedInputSubsystemInterface.AddMappingContext` _returnvalue "/Game/Pong/Inputs/Pong_IMC.Pong_IMC" 0 (struct))
      (bind _returnvalue_2 (`|CreateWidget` "/Game/Pong/Blueprints/PongScore_WB.PongScore_WB_C"))
      (bind _output_get (set `self.ScoreHUD` _returnvalue_2))
      (`UserWidget.AddToViewport` _output_get 0))))

(event `EnhancedInput|/Game/Pong/Inputs/PongMove_IA`
  (params (ActionValue :type "Float (double-precision)") (ElapsedSeconds :type "Float (double-precision)") (TriggeredSeconds :type "Float (double-precision)") (InputAction :type "InputAction Object Reference" :default "/Game/Pong/Inputs/PongMove_IA.PongMove_IA"))
  (:`Triggered`
    (`SceneComponent.K2_AddLocalOffset` (`self.Cube`) (`KismetMathLibrary.MakeVector` 0.0 (* ActionValue (`self.PlayerSpeed`))) true false)))

(fn `UserConstructionScript`)