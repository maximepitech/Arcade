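; PongGoal_BP is a goal in the Pong game that removes the ball and awards a point when the ball enters it.
; At BeginPlay it caches the player's paddle pawn to reach its ScoreHUD.
; A box overlap with the ball destroys it, and the PlayerGoal flag selects whether the HUD updates the AI's score (player's goal) or the player's score.
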(event `self.ReceiveBeginPlay`
  (bind _aspong_paddle_bp (cast `/Game/Pong/Blueprints/PongPaddle_BP` (`GameplayStatics.GetPlayerPawn` 0)))
  (set `self.As Pong Paddle BP` _aspong_paddle_bp))

(event `self.Box.OnComponentBeginOverlap`
  (params (OverlappedComponent :type "PrimitiveComponent Object Reference") (OtherActor :type "Actor Object Reference") (OtherComp :type "PrimitiveComponent Object Reference") (OtherBodyIndex :type Integer) (bFromSweep :type Boolean) (SweepResult :type "HitResult Structure (by ref)"))
  (bind _aspong_ball_bp (cast `/Game/Pong/Blueprints/PongBall_BP` OtherActor))
  (`self.K2_DestroyActor` _aspong_ball_bp)
  (if (`self.PlayerGoal?`)
    (`/Game/Pong/Blueprints/PongScore_WB.UpdateAIScore` (`/Game/Pong/Blueprints/PongPaddle_BP.ScoreHUD` (`self.As Pong Paddle BP`)))
    (else
      (`/Game/Pong/Blueprints/PongScore_WB.UpdatePlayerScore` (`/Game/Pong/Blueprints/PongPaddle_BP.ScoreHUD` (`self.As Pong Paddle BP`))))))

(fn `UserConstructionScript`)